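; BP_BlockingFog is a level blocker that removes itself once a designated set of enemies has died.
; On BeginPlay it binds EnemyCount to the death event of each HealthComponent on the actors in EnemyToDie.
; Each death increments EnemiesDead, and the fog destroys itself when that count reaches the length of the list.
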(event Custom|EnemyCount
  (bind _result (Math|Integer|IncrementInt (Variables|Default|GetEnemiesDead))
    (:%20%20
      (if (>= _result (Utilities|Array|Length (Variables|Default|GetEnemyToDie)))
        (Actor|DestroyActor)))))

(event EventBeginPlay
  (for _array_element (Variables|Default|GetEnemyToDie)
    (EventDispatchers|BindEventtoOnDeath (Actor|GetComponentbyClass _array_element "/Script/GP4.HealthComponent") (delegate Custom|EnemyCount))))

(fn ConstructionScript)