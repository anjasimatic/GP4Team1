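; Level actor that lights up an area once a set group of enemies has been killed.
; On BeginPlay it binds a counter to the death event of each HealthComponent in the EnemyToDie array.
; When the count reaches the array's length, a timeline plays and drives the intensity of its RectLight.
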(event Custom|EnemyCount
  (bind _result (Math|Integer|IncrementInt (Variables|Default|GetEnemiesDead))
    (:%20%20
      (if (>= _result (Utilities|Array|Length (Variables|Default|GetEnemyToDie)))
        (bind _newtrack_0 (Timeline|light_intensity PlayFromStart)
          (:Update
            (Rendering|Components|Light|SetIntensity (Variables|Default|GetRectLight) _newtrack_0)))))))

(event Collision|EventActorBeginOverlap
  (params (OtherActor :type Actor%20Object%20Reference)))

(event EventTick
  (params (DeltaSeconds :type Float%20%28single-precision%29)))

(event EventBeginPlay
  (for _array_element (Variables|Default|GetEnemyToDie)
    (EventDispatchers|BindEventtoOnDeath (Actor|GetComponentbyClass _array_element "/Script/GP4.HealthComponent") (delegate Custom|EnemyCount))))

(fn ConstructionScript)