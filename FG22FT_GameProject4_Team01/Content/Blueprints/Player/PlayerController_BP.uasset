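; Player controller that relays Enhanced Input actions to the player's GP4 character and toggles the pause menu.
; Movement, look, combat, targeting and ability actions pass their values to the character's input functions through GetValidCharacter, unforced.
; Button actions route press and release into the same call, with Block releasing on Canceled rather than Completed.
; Pause lazily creates and reuses WB_Pause, waiting one tick before closing it.
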(event Input|EnhancedActionEvents|EnhancedInputActionMove_IA
  (params (ActionValue :type Vector%202D%20Structure) (ElapsedSeconds :type Float%20%28double-precision%29) (TriggeredSeconds :type Float%20%28double-precision%29) (InputAction :type Input%20Action%20Object%20Reference :default "/Game/Blueprints/Player/Controls/Move_IA.Move_IA"))
  (:Triggered
    (bind _character (CallFunction|GetValidCharacter))
    (Class|GP4Character|MoveInput _character ActionValue false)))

(event Input|EnhancedActionEvents|EnhancedInputActionLook_IA
  (params (ActionValue :type Vector%202D%20Structure) (ElapsedSeconds :type Float%20%28double-precision%29) (TriggeredSeconds :type Float%20%28double-precision%29) (InputAction :type Input%20Action%20Object%20Reference :default "/Game/Blueprints/Player/Controls/Look_IA.Look_IA"))
  (:Triggered
    (bind _character (CallFunction|GetValidCharacter))
    (Class|GP4Character|LookInput _character ActionValue false)))

(event Input|EnhancedActionEvents|EnhancedInputActionAction_IA
  (params (ActionValue :type Boolean) (ElapsedSeconds :type Float%20%28double-precision%29) (TriggeredSeconds :type Float%20%28double-precision%29) (InputAction :type Input%20Action%20Object%20Reference :default "/Game/Blueprints/Player/Controls/Action_IA.Action_IA"))
  (:Started
    (bind _character (CallFunction|GetValidCharacter :!label _label))
    (Class|GP4Character|ActionInput _character ActionValue false))
  (:Completed
    (goto _label)))

(event Input|EnhancedActionEvents|EnhancedInputActionPause_IA
  (params (ActionValue :type Boolean) (ElapsedSeconds :type Float%20%28double-precision%29) (TriggeredSeconds :type Float%20%28double-precision%29) (InputAction :type Input%20Action%20Object%20Reference :default "/Game/Blueprints/Player/Controls/Pause_IA.Pause_IA"))
  (:Started
    (Utilities|IsValid (Variables|Default|GetPauseMenu)
      (:Is%20Valid
        (if (UserInterface|Viewport|IsinViewport (Variables|Default|GetPauseMenu))
          (Utilities|FlowControl|DelayUntilNextTick)
          (Default|CloseMenu (Variables|Default|GetPauseMenu))
          (else
            (UserInterface|Viewport|AddtoViewport (Variables|Default|GetPauseMenu) 0 :!label _label))))
      (:Is%20Not%20Valid
        (bind _returnvalue (UserInterface|CreateWidget "/Game/Blueprints/UI/WB_Pause.WB_Pause_C" self))
        (Variables|Default|SetPauseMenu _returnvalue)
        (goto _label)))))

(event Input|EnhancedActionEvents|EnhancedInputActionDodge_IA
  (params (ActionValue :type Boolean) (ElapsedSeconds :type Float%20%28double-precision%29) (TriggeredSeconds :type Float%20%28double-precision%29) (InputAction :type Input%20Action%20Object%20Reference :default "/Game/Blueprints/Player/Controls/Dodge_IA.Dodge_IA"))
  (:Started
    (bind _character (CallFunction|GetValidCharacter :!label _label))
    (Class|GP4Character|DodgeInput _character ActionValue false))
  (:Completed
    (goto _label)))

(event Input|EnhancedActionEvents|EnhancedInputActionTargetMode_IA
  (params (ActionValue :type Boolean) (ElapsedSeconds :type Float%20%28double-precision%29) (TriggeredSeconds :type Float%20%28double-precision%29) (InputAction :type Input%20Action%20Object%20Reference :default "/Game/Blueprints/Player/Controls/TargetMode_IA.TargetMode_IA"))
  (:Started
    (bind _character (CallFunction|GetValidCharacter :!label _label))
    (Class|GP4Character|CombatModeInput _character ActionValue false))
  (:Completed
    (goto _label)))

(event Input|EnhancedActionEvents|EnhancedInputActionTargetSwitch_IA
  (params (ActionValue :type Boolean) (ElapsedSeconds :type Float%20%28double-precision%29) (TriggeredSeconds :type Float%20%28double-precision%29) (InputAction :type Input%20Action%20Object%20Reference :default "/Game/Blueprints/Player/Controls/TargetSwitch_IA.TargetSwitch_IA"))
  (:Started
    (bind _character (CallFunction|GetValidCharacter :!label _label))
    (Class|GP4Character|TargetSwitchInput _character ActionValue false))
  (:Completed
    (goto _label)))

(event Input|EnhancedActionEvents|EnhancedInputActionStateSwitch_IA
  (params (ActionValue :type Boolean) (ElapsedSeconds :type Float%20%28double-precision%29) (TriggeredSeconds :type Float%20%28double-precision%29) (InputAction :type Input%20Action%20Object%20Reference :default "/Game/Blueprints/Player/Controls/StateSwitch_IA.StateSwitch_IA"))
  (:Triggered
    (bind _character (CallFunction|GetValidCharacter :!label _label))
    (Class|GP4Character|StateSwitchInput _character ActionValue false))
  (:Completed
    (goto _label)))

(event Input|EnhancedActionEvents|EnhancedInputActionAbility_IA
  (params (ActionValue :type Boolean) (ElapsedSeconds :type Float%20%28double-precision%29) (TriggeredSeconds :type Float%20%28double-precision%29) (InputAction :type Input%20Action%20Object%20Reference :default "/Game/Blueprints/Player/Controls/Ability_IA.Ability_IA"))
  (:Started
    (bind _character (CallFunction|GetValidCharacter :!label _label))
    (Class|GP4Character|AbilityInput _character ActionValue false))
  (:Completed
    (goto _label)))

(event Input|EnhancedActionEvents|EnhancedInputActionBlock_IA
  (params (ActionValue :type Boolean) (ElapsedSeconds :type Float%20%28double-precision%29) (TriggeredSeconds :type Float%20%28double-precision%29) (InputAction :type Input%20Action%20Object%20Reference :default "/Game/Blueprints/Player/Controls/Block_IA.Block_IA"))
  (:Started
    (bind _character (CallFunction|GetValidCharacter :!label _label))
    (Class|GP4Character|BlockInput _character ActionValue false))
  (:Canceled
    (goto _label)))

(fn ConstructionScript)

(fn GetValidCharacter
  (bind _returnvalue (Class|GP4PlayerController|GetGP4Character))
  (Utilities|IsValid _returnvalue
    (:Is%20Valid
      (return _returnvalue))))