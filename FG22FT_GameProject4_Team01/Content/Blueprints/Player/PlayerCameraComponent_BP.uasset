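; Player camera component that adapts camera pitch limits and automatic camera speed to the character's state.
; On a camera mode change, it sets the local camera manager's view pitch range to the Default or Combat preset.
; Each tick, it ramps the auto camera speed multiplier up while the character has movement acceleration and down while it has none, within a clamped range.
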(event EventTick
  (params (DeltaSeconds :type Float%20%28single-precision%29))
  (bind _returnvalue (Class|GP4CharacterCameraComponent|GetCharacterOwner))
  (Utilities|IsValid _returnvalue
    (:Is%20Valid
      (Utilities|FlowControl|Sequence
        (:then_0
          (bind _output_get (Variables|Default|SetCurrentAutoSpeedMulti (Math|Float|Clamp(Float) (+ (Variables|Default|GetCurrentAutoSpeedMulti) (* (Math|Float|SelectFloat -1.0 1.0 (Math|Vector|VectorIsNearlyZero (Pawn|Components|CharacterMovement|GetCurrentAcceleration (Variables|/Script/Engine.Character|GetCharacterMovement _returnvalue)))) DeltaSeconds)) 0.1)))
          (Variables|Default|SetAutoCameraSpeedMultiplier _output_get))))))

(event EventOnChangeCameraMode
  (params (NewMode :type EPlayerCameraMode%20Enum :default "Default"))
  (bind _defaultpitchrange (Variables|Default|GetDefaultPitchRange))
  (bind _combatpitchrange (Variables|Default|GetCombatPitchRange))
  (bind _returnvalue (Utilities|Select :Index NewMode :Default _defaultpitchrange :Combat _combatpitchrange))
  (bind (_x _y) (Math|Vector2D|BreakVector2D _returnvalue))
  (bind _ascharacter (Utilities|Casting|CastToCharacter (Class|GP4CharacterCameraComponent|GetPawnOwner)))
  (Variables|/Script/Engine.PlayerCameraManager|SetViewPitchMin (Variables|/Script/Engine.PlayerController|GetPlayerCameraManager (Pawn|GetLocalViewingPlayerController _ascharacter)) _x)
  (Variables|/Script/Engine.PlayerCameraManager|SetViewPitchMax (Variables|/Script/Engine.PlayerController|GetPlayerCameraManager (Pawn|GetLocalViewingPlayerController _ascharacter)) _y))